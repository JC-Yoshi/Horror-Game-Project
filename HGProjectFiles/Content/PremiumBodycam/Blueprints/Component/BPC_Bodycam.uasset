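; Actor component that gives the player camera a bodycam look through post-process settings, FOV, a screen blur widget and material parameter collections.
; Its tick function picks idle, walk or run camera shakes by character speed.
; It also wobbles the vignette via MPC_Vignette, using interpolated camera rotation deltas plus random jitter while moving.
; Helper functions drive blur amount through MPC_Blur and set vignette intensity on the camera.
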(fn InitilizeBodycam
  (params (Player%20Camera :type Camera%20Component%20Object%20Reference) (FieldOfView :type Float%20%28single-precision%29) (Focal%20Distance :type Float%20%28single-precision%29) (Bloom%20Method :type EBloomMethod%20Enum :default "BM_SOG") (Chromatic%20Aberration%20Intensity :type Float%20%28single-precision%29) (Lens%20Dirt%20Texture :type Texture%20Object%20Reference) (Lens%20Dirt%20Intensity :type Float%20%28single-precision%29) (Min%20Exposure :type Float%20%28single-precision%29) (Max%20Exposure :type Float%20%28single-precision%29) (Exposure%20Compensation :type Float%20%28single-precision%29) (Exposure%20Adaptation%20Speed :type Float%20%28single-precision%29) (Grain%20Intensity :type Float%20%28single-precision%29) (Grain%20Size :type Float%20%28single-precision%29))
  (Utilities|Struct|SetmembersinPostProcessSettings (Variables|/Script/Engine.CameraComponent|GetPostProcessSettings Player%20Camera) Bloom%20Method (Variables|PostProcessSettings|GetGlobal%20Contrast) (Variables|PostProcessSettings|GetShadowContrast) (Variables|PostProcessSettings|GetHighlightContrast) Chromatic%20Aberration%20Intensity Lens%20Dirt%20Texture Lens%20Dirt%20Intensity Exposure%20Compensation Min%20Exposure Max%20Exposure Exposure%20Adaptation%20Speed Exposure%20Adaptation%20Speed Grain%20Intensity Grain%20Size Focal%20Distance (Variables|AdditionalSettings|GetPost%20Process%20Materials))
  (CallFunction|InitilizeWidgets)
  (Camera|SetFieldOfView Player%20Camera FieldOfView)
  (Rendering|Material|SetScalarParameterValue "/Game/PremiumBodycam/Materials/PostProcess/BaseMaterials/MPC_Blur.MPC_Blur" "BlurAmount" 0.0 :!class /Script/Engine.KismetMaterialLibrary))

(fn InitilizeWidgets
  (bind _returnvalue (UserInterface|CreateWidget "/Game/PremiumBodycam/Widgets/W_ScreenBlur.W_ScreenBlur_C"))
  (bind _output_get (Variables|AdditionalSettings|SetScreen%20Blur%20Ref _returnvalue))
  (UserInterface|Viewport|AddtoViewport _output_get 0))

(fn InitilizeEventTick
  (params (Player%20Camera :type Scene%20Component%20Object%20Reference))
  (bind _returnvalue (Transformation|GetWorldRotation Player%20Camera))
  (bind _returnvalue_2 (Utilities|Time|GetWorldDeltaSeconds))
  (bind _returnvalue_3 (Utilities|Time|GetWorldDeltaSeconds))
  (bind _returnvalue_4 (Utilities|Time|GetWorldDeltaSeconds))
  (bind _returnvalue_5 (Utilities|Time|GetWorldDeltaSeconds))
  (bind _yawrateminmax (Variables|AdditionalSettings|GetYawRateMinMax))
  (bind _pitchrateminmax (Variables|AdditionalSettings|GetPitchRateMinMax))
  (bind (_roll _pitch _yaw) (Math|Rotator|BreakRotator _returnvalue))
  ;[1 1 1] Vignette Wobble
  (Utilities|FlowControl|Sequence
    (:then_0
      (CallFunction|UpdateCameraShake))
    (:then_1
      (Variables|AdditionalSettings|SetPitchRate (Math|Float|Clamp(Float) (+ (Variables|AdditionalSettings|GetPitchRate) (- _pitch (.pitch (Variables|AdditionalSettings|GetCamRotator)))) (* _pitchrateminmax -1.0) _pitchrateminmax))
      (Variables|AdditionalSettings|SetYawRate (Math|Float|Clamp(Float) (+ (Variables|AdditionalSettings|GetYawRate) (- _yaw (.yaw (Variables|AdditionalSettings|GetCamRotator)))) (* _yawrateminmax -1.0) _yawrateminmax))
      (Variables|AdditionalSettings|SetCamRotator _returnvalue)
      (bind _output_get (Variables|AdditionalSettings|SetPitch%20Vignette%20Offset (Math|Interpolation|FInterpTo (Variables|AdditionalSettings|GetPitch%20Vignette%20Offset) (Variables|AdditionalSettings|GetPitchRate) _returnvalue_2 1e+01)))
      (bind _output_get_2 (Variables|AdditionalSettings|SetYaw%20Vignette%20Offset (Math|Interpolation|FInterpTo (Variables|AdditionalSettings|GetYaw%20Vignette%20Offset) (Variables|AdditionalSettings|GetYawRate) _returnvalue_2 1e+01)))
      (Rendering|Material|SetVectorParameterValue "/Game/PremiumBodycam/Materials/PostProcess/BaseMaterials/MPC_Vignette.MPC_Vignette" "VignetteOffset" (Utilities|Struct|MakeLinearColor _output_get_2 _output_get 0.0 1.0) :!class /Script/Engine.KismetMaterialLibrary)
      (Variables|AdditionalSettings|SetYawRate (Math|Interpolation|FInterpTo (Variables|AdditionalSettings|GetYawRate) 0.0 (Utilities|Time|GetWorldDeltaSeconds) 15.0))
      (Variables|AdditionalSettings|SetPitchRate (Math|Interpolation|FInterpTo (Variables|AdditionalSettings|GetPitchRate) 0.0 (Utilities|Time|GetWorldDeltaSeconds) 15.0)))
    (:then_2
      (if (>= (Math|Vector|VectorLength (Transformation|GetVelocity (Game|GetPlayerCharacter 0))) 8e+01)
        ;[1 1 1] Vignette Shake
        (Variables|AdditionalSettings|SetPitch%20Shake (Math|Interpolation|FInterpTo (Variables|AdditionalSettings|GetPitch%20Shake) (Math|Random|RandomFloatinRange -1e+01 1e+01) _returnvalue_5 3.0))
        (Variables|AdditionalSettings|SetYaw%20Shake (Math|Interpolation|FInterpTo (Variables|AdditionalSettings|GetYaw%20Shake) (Math|Random|RandomFloatinRange -1e+01 1e+01) _returnvalue_5 3.0))
        (bind _output_get_3 (Variables|AdditionalSettings|SetPitch%20Vignette%20Shake (Math|Interpolation|FInterpTo (Variables|AdditionalSettings|GetPitch%20Vignette%20Shake) (Variables|AdditionalSettings|GetPitch%20Shake) _returnvalue_3 2e+01)))
        (bind _output_get_4 (Variables|AdditionalSettings|SetYaw%20Vignette%20Shake (Math|Interpolation|FInterpTo (Variables|AdditionalSettings|GetYaw%20Vignette%20Shake) (Variables|AdditionalSettings|GetYaw%20Shake) _returnvalue_3 2e+01)))
        (Rendering|Material|SetVectorParameterValue "/Game/PremiumBodycam/Materials/PostProcess/BaseMaterials/MPC_Vignette.MPC_Vignette" "VignetteShake" (Utilities|Struct|MakeLinearColor _output_get_4 _output_get_3 0.0 1.0) :!class /Script/Engine.KismetMaterialLibrary)
        (Variables|AdditionalSettings|SetPitch%20Vignette%20Shake (Math|Interpolation|FInterpTo (Variables|AdditionalSettings|GetPitch%20Shake) 0.0 _returnvalue_4 2e+01))
        (Variables|AdditionalSettings|SetYaw%20Vignette%20Shake (Math|Interpolation|FInterpTo (Variables|AdditionalSettings|GetYaw%20Shake) 0.0 _returnvalue_4 2e+01))))))

(fn UpdateCameraShake
  (bind _returnvalue (Game|GetPlayerCharacter 0))
  (bind _returnvalue_2 (Game|GetPlayerController 0))
  (if (<= (Math|Vector|VectorLength (Transformation|GetVelocity _returnvalue)) 99.0)
    (Game|Feedback|ClientStartCameraShake _returnvalue_2 "/Game/PremiumBodycam/Blueprints/CameraShakes/Bodycam/CS_Idle.CS_Idle_C" 1.0 "CameraLocal" "0, 0, 0")
    (elif (>= (Math|Vector|VectorLength (Transformation|GetVelocity _returnvalue)) 5e+02)
      (Game|Feedback|ClientStartCameraShake _returnvalue_2 "/Game/PremiumBodycam/Blueprints/CameraShakes/Bodycam/CS_Run.CS_Run_C" 1.0 "CameraLocal" "0, 0, 0")
      (else
        (Game|Feedback|ClientStartCameraShake _returnvalue_2 "/Game/PremiumBodycam/Blueprints/CameraShakes/Bodycam/CS_Walk.CS_Walk_C" 1.0 "CameraLocal" "0, 0, 0")))))

(fn ActionBlur
  (params (Alpha :type Float%20%28single-precision%29))
  (Rendering|Material|SetScalarParameterValue "/Game/PremiumBodycam/Materials/PostProcess/BaseMaterials/MPC_Blur.MPC_Blur" "BlurAmount" Alpha :!class /Script/Engine.KismetMaterialLibrary))

(fn FocusVignette
  (params (Player%20Camera :type Camera%20Component%20Object%20Reference) (Vignette%20Intensity :type Float%20%28single-precision%29))
  (Utilities|Struct|SetmembersinPostProcessSettings (Variables|/Script/Engine.CameraComponent|GetPostProcessSettings Player%20Camera) Vignette%20Intensity))