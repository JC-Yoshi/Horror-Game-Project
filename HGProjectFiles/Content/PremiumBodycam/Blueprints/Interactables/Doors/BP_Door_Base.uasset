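; Base interactable door that the player pushes open with physics and that closes through a timeline, with open, close and locked sounds.
; Interact enables physics simulation and applies an impulse along the player's forward vector, or disables physics and lerps the yaw shut using a computed close direction.
; When locked, Interact instead plays a yaw timeline with a locked sound.
; TriggerOpenDoor and TriggerCloseDoor allow scripted unlocking, directional pushes, and closing with optional locking.
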(event Custom|CloseDoor
  (bind _doorframe (Variables|Default|GetDoorFrame))
  (bind _door (Variables|Default|GetDoor))
  (bind _returnvalue (Transformation|GetWorldRotation _doorframe))
  (bind _relativerotation (Variables|/Script/Engine.SceneComponent|GetRelativeRotation _door))
  ;[0.025 0.025 0.025] Close Door Event
  (Utilities|FlowControl|Sequence
    (:then_0
      (Physics|SetSimulatePhysics (Variables|Default|GetDoor) false)
      (bind _alpha (Timeline|Door_TL PlayFromStart)
        (:Update
          (Transformation|SetRelativeRotation _door (Math|Rotator|MakeRotator (.roll _relativerotation) (.pitch _relativerotation) (Math|Float|Lerp (.yaw _relativerotation) (Math|Float|SelectFloat (* (.yaw _returnvalue) -1.0) (.yaw _returnvalue) (CallFunction|CalculateCloseDirection)) _alpha)) false false))))
    (:then_1
      (Utilities|FlowControl|Delay 0.2)
      (Variables|Default|SetDoorOpen false)
      (CallFunction|Reset)
      (bind _returnvalue_2 (Audio|SpawnSoundatLocation (Variables|Default|GetCloseSound) (Transformation|GetActorLocation) "0, 0, 0" 1.0 1.0 0.0 0 0))
      (Components|Activation|SetActive _returnvalue_2 true (Audio|Components|Audio|IsPlaying _returnvalue_2)))))

(event Custom|StopTL
  (bind _doorframe (Variables|Default|GetDoorFrame))
  (bind _door (Variables|Default|GetDoor))
  (bind _returnvalue (Transformation|GetWorldRotation _doorframe))
  (bind _relativerotation (Variables|/Script/Engine.SceneComponent|GetRelativeRotation _door))
  ;[0.025 0.025 0.025] Close Door Event
  (bind _alpha (Timeline|Door_TL Stop)
    (:Update
      (Transformation|SetRelativeRotation _door (Math|Rotator|MakeRotator (.roll _relativerotation) (.pitch _relativerotation) (Math|Float|Lerp (.yaw _relativerotation) (Math|Float|SelectFloat (* (.yaw _returnvalue) -1.0) (.yaw _returnvalue) (CallFunction|CalculateCloseDirection)) _alpha)) false false))))

(event Custom|Reset
  ;[0.025 0.025 0.025] Interact Event
  (Utilities|FlowControl|Sequence
    (:then_0
      (Utilities|FlowControl|DoOnce false) ; enters at Reset
    )
    (:then_1
      (Utilities|IsValid (stale EventInteract _returnvalue)
        (:Is%20Valid
          (Components|Activation|SetActive (stale EventInteract _returnvalue) false (Audio|Components|Audio|IsPlaying (stale EventInteract _returnvalue))))))))

(event Custom|TriggerCloseDoor
  (params (Lock :type Boolean))
  ;[0.025 0.025 0.025] Trigger Open/Close Events
  (CallFunction|CloseDoor)
  (Variables|Default|SetWasUnlocked true)
  (if Lock
    (Variables|Default|SetLocked true)))

(event Custom|LockedCheck
  (bind _door (Variables|Default|GetDoor))
  (bind _relativerotation (Variables|/Script/Engine.SceneComponent|GetRelativeRotation _door))
  ;[0.025 0.025 0.025] Locked Event
  (Utilities|FlowControl|Sequence
    (:then_0
      (if (not (Audio|Components|Audio|IsPlaying (Variables|Default|GetLocked_TL)))
        (bind _alpha (Timeline|Locked_TL PlayFromStart)
          (:Update
            (Transformation|SetRelativeRotation _door (Math|Rotator|MakeRotator (.roll _relativerotation) (.pitch _relativerotation) (Math|Float|SelectFloat (+ (.yaw (Transformation|GetWorldRotation (Variables|Default|GetDoorFrame))) _alpha) _alpha (Variables|Default|GetWasUnlocked))) false false)))
        (else
          (Timeline|Locked_TL Reverse))))
    (:then_1
      (bind _returnvalue (Audio|SpawnSoundatLocation (Variables|Default|GetLockedSound) (Transformation|GetActorLocation) "0, 0, 0" 1.0 1.0 0.0 0 0))
      (Components|Activation|SetActive _returnvalue true (Audio|Components|Audio|IsPlaying _returnvalue)))))

(event Custom|TriggerOpenDoor
  (params (OpenForward :type Boolean) (OpenImpulse :type Float%20%28single-precision%29))
  (bind _door (Variables|Default|GetDoor))
  (bind _targetforward (Variables|Default|GetTargetForward))
  (bind _targetbackward (Variables|Default|GetTargetBackward))
  ;[0.025 0.025 0.025] Trigger Open/Close Events
  (if (Variables|Default|GetLocked)
    (Variables|Default|SetLocked false))
  (CallFunction|Interact)
  (if OpenForward
    (Physics|AddImpulseatLocation _door (* (Math|Vector|GetForwardVector _targetforward) OpenImpulse) (Transformation|GetWorldLocation _targetforward) "None")
    (else
      (Physics|AddImpulseatLocation _door (* (Math|Vector|GetForwardVector _targetbackward) OpenImpulse) (Transformation|GetWorldLocation _targetbackward) "None"))))

(event EventInteract
  ;[0.025 0.025 0.025] Interact Event
  (if (not (Variables|Default|GetLocked))
    (if (not (Variables|Default|GetDoorOpen))
      (if (Audio|Components|Audio|IsPlaying (Variables|Default|GetDoor_TL))
        (CallFunction|StopTL)
        (Utilities|FlowControl|Sequence
          (:then_0
            (goto _label Reset))
          (:then_1
            _)))
      (Utilities|FlowControl|DoOnce false :!label _label
        (:Completed
          (Physics|SetSimulatePhysics (Variables|Default|GetDoor) true)
          (Physics|AddImpulseatLocation (Variables|Default|GetDoor) (* (Transformation|GetActorForwardVector (Game|GetPlayerCharacter 0)) (Variables|Default|GetOpenImpulse)) (Transformation|GetWorldLocation (Variables|Default|GetDoorFrame)) "None")
          (Variables|Default|SetDoorOpen true)
          (bind _returnvalue (Audio|SpawnSoundatLocation (Variables|Default|GetOpenSound) (Transformation|GetActorLocation) "0, 0, 0" 1.0 1.0 0.0 0 0))
          (Components|Activation|SetActive _returnvalue true false)))
      (else
        (CallFunction|CloseDoor)))
    (else
      (CallFunction|LockedCheck))))

(fn ConstructionScript)

(fn CalculateCloseDirection
  (bind _doorframe (Variables|Default|GetDoorFrame))
  (bind _returnvalue (Transformation|GetWorldRotation _doorframe))
  (return (> (Math|Vector|DotProduct (Math|Conversions|ToVector(Float) (Math|Rotator|NormalizeAxis (- (.yaw (Variables|/Script/Engine.SceneComponent|GetRelativeRotation (Variables|Default|GetDoor))) (Math|Float|SelectFloat (.yaw (Variables|/Script/Engine.SceneComponent|GetRelativeRotation _doorframe)) (.yaw _returnvalue) (> (.yaw _returnvalue) 9e+01))))) (Math|Vector|GetForwardVector _doorframe)) 0.0)))